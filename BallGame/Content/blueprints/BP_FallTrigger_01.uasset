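; BP_FallTrigger_01 is a trigger actor that restarts the current level when an overlap with its FallTriger component ends.
; BeginPlay fades the first player's camera in from opaque.
; End overlap, with no check on which actor left, fades the camera out and holds it, then reopens the current level by name after a delay.
; An unconnected node that would open "main" never runs.
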(event OnComponentEndOverlap(falltriger)
  (params (OverlappedComponent :type Primitive%20Component%20Object%20Reference) (OtherActor :type Actor%20Object%20Reference) (OtherComp :type Primitive%20Component%20Object%20Reference) (OtherBodyIndex :type Integer))
  (bind _returnvalue (Game|GetCurrentLevelName true))
  (CameraFades|StartCameraFade :self (Variables|/Script/Engine.PlayerController|GetPlayerCameraManager (Game|GetPlayerController 0)) :ToAlpha 1.0 :Duration 2.0 :bHoldWhenFinished true)
  (Utilities|FlowControl|Delay 3.0)
  (Game|OpenLevel(byName) (Utilities|String|StringToName _returnvalue)))

(event EventBeginPlay
  (CameraFades|StartCameraFade :self (Variables|/Script/Engine.PlayerController|GetPlayerCameraManager (Game|GetPlayerController 0)) :FromAlpha 1.0 :Duration 2.0))

(fn ConstructionScript)