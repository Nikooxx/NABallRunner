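; BP_Ball_02 is a player-controlled ball that rolls by physics torque and can jump.
; Up/Down and Left/Right axis inputs apply torque to the Sphere around Y and X, scaled by Multiply as an acceleration change.
; Space bar plays the Jump timeline, which repositions the Sphere each update at the actor's location plus a scaled curve Z offset.
; BeginPlay fades the player camera in from opaque.
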(event EventBeginPlay
  (CameraFades|StartCameraFade :self (Variables|/Script/Engine.PlayerController|GetPlayerCameraManager (Game|GetPlayerController 0)) :FromAlpha 1.0 :Duration 2.0))

(event Input|AxisEvents|InputAxisUp/Down
  (params (AxisValue :type Float%20%28single-precision%29))
  (Class|PrimitiveComponent|AddTorqueinDegrees (Variables|Default|GetSphere) (Math|Vector|MakeVector 0.0 (* AxisValue (Variables|Default|Getmultiply)) 0.0) "None" true))

(event Input|AxisEvents|InputAxisLeft/Right
  (params (AxisValue :type Float%20%28single-precision%29))
  (Class|PrimitiveComponent|AddTorqueinDegrees (Variables|Default|GetSphere) (Math|Vector|MakeVector (* AxisValue (Variables|Default|Getmultiply)) 0.0 0.0) "None" true))

(event Input|KeyboardEvents|SpaceBar
  (params (Key :type Key%20Structure :default "None"))
  (bind _returnvalue (Transformation|GetActorLocation))
  (:Pressed
    (bind _jump (Timeline|Jump PlayFromStart)
      (:Update
        (Transformation|SetWorldLocation (Variables|Default|GetSphere) (Math|Vector|MakeVector (.x _returnvalue) (.y _returnvalue) (+ (* (.z _jump) 1e+01) (.z _returnvalue))) false false)))))

(fn ConstructionScript)